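; Skill tree manager that creates skill objects and tracks which skill classes are unlocked.
; SpawnSkills constructs an object from each class in Skills and stores it in SkillReferences.
; UnlockSkill adds a skill's class to UnlockedSkills only when its UnlockDependencies array is identical to the whole UnlockedSkills array, rather than merely contained in it.
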(fn SpawnSkills
  (for _array_element (Variables|Default|GetSkills)
    (bind _returnvalue (Game|ConstructObjectfromClass _array_element))
    (Utilities|Array|Add (Variables|Default|GetSkillReferences) _returnvalue)))

(fn UnlockSkill
  (params (Skill :type BP%20Skill%20Object%20Reference))
  (if (Utilities|Array|Identical (.unlockdependencies (Variables|/Game/Blueprints/BP_Skill.BP_Skill_C|GetSkillData Skill)) (Variables|Default|GetUnlockedSkills))
    (Utilities|Array|Add (Variables|Default|GetUnlockedSkills) (Utilities|GetClass Skill))))